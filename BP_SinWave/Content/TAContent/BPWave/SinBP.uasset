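; SinBP is a construction-script actor that builds a sine-wave visual from a row of static mesh strips spaced along X.
; A loop spawns each strip and passes sine force range, a random factor, color and point count to its materials.
; Four sphere components act as control handles, with Y mapped to normalized position and Z to wave strength.
; An index-based ratio scales strength and color, and the wave shaping itself is left to the material.
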(event `self.ReceiveTick`
  (params (DeltaSeconds :type "Float (single-precision)")))

(fn `UserConstructionScript`
  (bind _index (`self.Index`))
  (bind _forcemax_z (`self.ForceMax(Z`))
  (bind (_relativelocation_x _relativelocation_y _relativelocation_z) (`KismetMathLibrary.BreakVector` (`SceneComponent.RelativeLocation` (`self.Sphere2`))))
  (bind (_relativelocation_x_2 _relativelocation_y_2 _relativelocation_z_2) (`KismetMathLibrary.BreakVector` (`SceneComponent.RelativeLocation` (`self.Sphere3`))))
  (bind (_relativelocation_x_3 _relativelocation_y_3 _relativelocation_z_3) (`KismetMathLibrary.BreakVector` (`SceneComponent.RelativeLocation` (`self.Sphere4`))))
  (bind (_relativelocation_x_4 _relativelocation_y_4 _relativelocation_z_4) (`KismetMathLibrary.BreakVector` (`SceneComponent.RelativeLocation` (`self.Sphere1`))))
  (for _index_2 (range 1 (+ _index 1))
    (bind _returnvalue (`AddComponent|NODE_AddStaticMeshComponent-0` :`RelativeTransform` (`KismetMathLibrary.MakeTransform` (`KismetMathLibrary.MakeVector` (`KismetMathLibrary.Conv_IntToDouble` (* (- _index_2 1) (`self.Distance`)))) (struct) (`KismetMathLibrary.MakeVector` 1.0 1.0 (* (`self.Weight`) 0.002)))))
    (`MeshComponent.SetVectorParameterValueOnMaterials` _returnvalue "BP" (`KismetMathLibrary.MakeVector` (`self.SinForceMin`) (`self.SinForceMax`) (`KismetMathLibrary.RandomFloatInRange` 1.0 3.0)))
    (`MeshComponent.SetScalarParameterValueOnMaterials` _returnvalue "Postion1" (/ (+ _relativelocation_y_4 -710.0 0.0) -1420.0))
    (bind _returnvalue_2 (/ (`KismetMathLibrary.Conv_IntToDouble` (+ (- _index _index_2) 1)) (`KismetMathLibrary.Conv_IntToDouble` _index)))
    (`MeshComponent.SetScalarParameterValueOnMaterials` _returnvalue "Value1" (* (/ _relativelocation_z_4 _forcemax_z) _returnvalue_2))
    (`MeshComponent.SetVectorParameterValueOnMaterials` _returnvalue "Color" (* (`KismetMathLibrary.Conv_LinearColorToVector` (* (`KismetMathLibrary.Conv_ColorToLinearColor` (`self.Color`)) _returnvalue_2)) 20.0))
    (`MeshComponent.SetScalarParameterValueOnMaterials` _returnvalue "Postion2" (/ (+ _relativelocation_y -710.0 0.0) -1420.0))
    (`MeshComponent.SetScalarParameterValueOnMaterials` _returnvalue "Value2" (* _returnvalue_2 (/ _relativelocation_z _forcemax_z)))
    (`MeshComponent.SetScalarParameterValueOnMaterials` _returnvalue "Postion3" (/ (+ _relativelocation_y_2 -710.0 0.0) -1420.0))
    (`MeshComponent.SetScalarParameterValueOnMaterials` _returnvalue "Value3" (* _returnvalue_2 (/ _relativelocation_z_2 _forcemax_z)))
    (`MeshComponent.SetScalarParameterValueOnMaterials` _returnvalue "Postion4" (/ (+ _relativelocation_y_3 -710.0 0.0) -1420.0))
    (`MeshComponent.SetScalarParameterValueOnMaterials` _returnvalue "Value4" (* _returnvalue_2 (/ _relativelocation_z_3 _forcemax_z)))
    (`MeshComponent.SetScalarParameterValueOnMaterials` _returnvalue "pointCount" (`self.WaveRange`))))